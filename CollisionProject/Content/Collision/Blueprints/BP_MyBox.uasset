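; BP_MyBox is a collision test actor whose Cube2 component acts as a trigger for motion on other objects.
; On begin overlap it prints the components and actor involved, then fires PlayCustomEvent on every MoveRect element, PlayRotationBall on RotationB and PlayMoveLeftRight on NewVar0.
; End overlap and hit events are empty; disconnected leftover graphs hold loop print tests and duplicate-filtered debug logging.
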(event OnComponentBeginOverlap(Cube2)
  (params (OverlappedComponent :type Primitive%20Component%20Object%20Reference) (OtherActor :type Actor%20Object%20Reference) (OtherComp :type Primitive%20Component%20Object%20Reference) (OtherBodyIndex :type Integer) (bFromSweep :type Boolean) (SweepResult :type Hit%20Result%20Structure%20%28by%20ref%29))
  (Development|PrintString (Utilities|String|Append "Overlappedcomponent=" (Utilities|GetDisplayName OverlappedComponent) "otherActor=" (Utilities|GetDisplayName OtherActor) "OtherComponent=" (Utilities|GetDisplayName OtherComp)) true true "(R=0.000000,G=0.660000,B=1.000000,A=1.000000)" 2e+02)
  (for _array_element (Variables|Default|GetmoveRect)
    (Default|PlayCustomEvent _array_element))
  (Default|PlayRotationBall (Variables|Default|GetRotationB))
  (Default|PlayMoveLeftRight (Variables|Default|GetNewVar_0)))

(event OnComponentEndOverlap(Cube2)
  (params (OverlappedComponent :type Primitive%20Component%20Object%20Reference) (OtherActor :type Actor%20Object%20Reference) (OtherComp :type Primitive%20Component%20Object%20Reference) (OtherBodyIndex :type Integer)))

(event OnComponentHit(Cube2)
  (params (HitComponent :type Primitive%20Component%20Object%20Reference) (OtherActor :type Actor%20Object%20Reference) (OtherComp :type Primitive%20Component%20Object%20Reference) (NormalImpulse :type Vector :default "0, 0, 0") (Hit :type Hit%20Result%20Structure%20%28by%20ref%29)))

(event EventBeginPlay)

(event Collision|EventActorBeginOverlap
  (params (OtherActor :type Actor%20Object%20Reference)))

(event EventTick
  (params (DeltaSeconds :type Float%20%28single-precision%29)))

(fn ConstructionScript)