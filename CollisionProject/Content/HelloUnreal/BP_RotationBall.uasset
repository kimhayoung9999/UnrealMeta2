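; BP_RotationBall is a Blueprint that swings its Scene component in roll while a BP_MyBox overlap is active.
; On BeginPlay it binds to the begin and end overlap dispatchers of every BP_MyBox, which start and stop the motion.
; A timeline drives the roll, flipping IsMoveRight on finish to alternate playing forward and reverse.
; Tick also gathers all boxes each frame but does nothing with them.
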(event EventBeginPlay
  (bind _outactors (Actor|GetAllActorsOfClass "/Game/Collision/Blueprints/BP_MyBox.BP_MyBox_C"))
  (for _array_element _outactors
    (EventDispatchers|BindEventtoNewEventDispatcherBeginOverLap _array_element (EventDispatchers|CreateEvent :!event EventBeginOverLap))
    (EventDispatchers|BindEventtoNewEventDispatcherEndOverLap _array_element (EventDispatchers|CreateEvent :!event EventEndOverLap))))

(event EventStop
  (bind _value (Timeline|타임라인_0 Stop)
    (:Update
      (Transformation|SetRelativeRotation (Variables|Default|GetScene) (Math|Rotator|MakeRotator (* _value 45.0) 0.0 0.0) false false))
    (:Finished
      (Variables|Default|SetIsMoveRight (not (Variables|Default|GetIsMoveRight)))
      (if (Variables|Default|GetIsMoveRight)
        (Timeline|타임라인_0 Play)
        (else
          (Timeline|타임라인_0 Reverse))))))

(event EventPlay
  (if (Variables|Default|GetIsMoveRight) :!label _label
    (bind _value (Timeline|타임라인_0 Play)
      (:Update
        (Transformation|SetRelativeRotation (Variables|Default|GetScene) (Math|Rotator|MakeRotator (* _value 45.0) 0.0 0.0) false false))
      (:Finished
        (Variables|Default|SetIsMoveRight (not (Variables|Default|GetIsMoveRight)))
        (goto _label)))
    (else
      (Timeline|타임라인_0 Reverse))))

(event EventTick
  (params (DeltaSeconds :type Float%20%28single-precision%29))
  (bind _outactors (Actor|GetAllActorsOfClass "/Game/Collision/Blueprints/BP_MyBox.BP_MyBox_C"))
  (for _array_element _outactors
    _))

(fn ConstructionScript)

(fn EventBeginOverLap
  (params (BeResult :type Boolean))
  (CallFunction|Play))

(fn EventEndOverLap
  (params (NewParam :type Boolean))
  (CallFunction|Stop))