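; BP_MoveLeftRight is an actor that slides its static mesh back and forth along X in response to BP_MyBox overlaps.
; BeginPlay binds to begin- and end-overlap dispatchers on every BP_MyBox, with overlap handlers that call Play and Stop.
; A timeline drives relative location, flipping ISMoveRight when finished to alternate Play and Reverse.
; A roll-rotation variant is unconnected, and Tick gathers boxes without acting on them.
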(event EventBeginPlay
  (bind _outactors (Actor|GetAllActorsOfClass "/Game/Collision/Blueprints/BP_MyBox.BP_MyBox_C"))
  (for _array_element _outactors
    (EventDispatchers|BindEventtoNewEventDispatcherBeginOverLap _array_element (EventDispatchers|CreateEvent :!event EventBeginOverlap))
    (EventDispatchers|BindEventtoNewEventDispatcherEndOverLap _array_element (EventDispatchers|CreateEvent :!event EventEndOverLap))))

(event EventTick
  (params (DeltaSeconds :type Float%20%28single-precision%29))
  (bind _outactors (Actor|GetAllActorsOfClass "/Game/Collision/Blueprints/BP_MyBox.BP_MyBox_C"))
  (for _array_element _outactors
    _))

(event EventStop
  (bind _value (Timeline|타임라인_0 Stop)
    (:Update
      (Transformation|SetRelativeLocation (Variables|Default|GetStaticMesh) (Math|Vector|MakeVector (* _value 1e+03) 0.0 0.0) false false))
    (:Finished
      (Variables|Default|SetISMoveRight (not (Variables|Default|GetISMoveRight)))
      (if (Variables|Default|GetISMoveRight)
        (Timeline|타임라인_0 Play)
        (else
          (Timeline|타임라인_0 Reverse))))))

(event EventPlay
  (if (Variables|Default|GetISMoveRight) :!label _label
    (bind _value (Timeline|타임라인_0 Play)
      (:Update
        (Transformation|SetRelativeLocation (Variables|Default|GetStaticMesh) (Math|Vector|MakeVector (* _value 1e+03) 0.0 0.0) false false))
      (:Finished
        (Variables|Default|SetISMoveRight (not (Variables|Default|GetISMoveRight)))
        (goto _label)))
    (else
      (Timeline|타임라인_0 Reverse))))

(fn ConstructionScript)

(fn NewFunction0
  (params (NewParam :type Boolean))
  (return))

(fn EventBeginOverlap
  (params (BeResult :type Boolean))
  (CallFunction|Play))

(fn EventEndOverLap
  (params (NewParam :type Boolean))
  (CallFunction|Stop))