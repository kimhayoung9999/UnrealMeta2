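; BP_P38 is an actor, apparently a P-38 aircraft, that flies in a straight line with two spinning propellers.
; Each Tick, a shared RotatePropeller function applies delta-time-scaled world roll to both propeller meshes at the Speed variable's rate.
; Tick also moves the actor along world +X at a fixed, frame-rate-independent speed, without sweep, so movement ignores collision and the actor's facing.
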(event EventBeginPlay)

(event Collision|EventActorBeginOverlap
  (params (OtherActor :type Actor%20Object%20Reference)))

(event EventTick
  (params (DeltaSeconds :type Float%20%28single-precision%29))
  (CallFunction|RotatePropeller (Variables|Default|GetStaticMesh2))
  (CallFunction|RotatePropeller (Variables|Default|GetStaticMesh1))
  (Transformation|AddActorWorldOffset (Math|Vector|MakeVector (* (Utilities|Time|GetWorldDeltaSeconds) 3.6e+02) 0.0 0.0)))

(fn ConstructionScript)

(fn RotatePropeller
  (params (self2 :type Scene%20Component%20Object%20Reference))
  (Transformation|AddWorldRotation self2 (Math|Rotator|MakeRotator (* (Utilities|Time|GetWorldDeltaSeconds) (Variables|Default|GetSpeed)) 0.0 0.0) false false))